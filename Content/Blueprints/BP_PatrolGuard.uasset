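; BP_PatrolGuard is a guard character that shows its alert state on a widget.
; On a state change it calls the parent handler, then sets the WBP_GuardState text to blank, "?" or "!" for Idle, Suspicious or Alerted.
; BeginPlay and overlap only forward to the parent.
; Logic for moving between BP_GuardPatrolZone actors and stopping on alert remains in the graph but is disconnected.
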(event EventBeginPlay
  (|CallParentFunction))

(event Collision|EventActorBeginOverlap
  (params (OtherActor :type Actor%20Object%20Reference))
  (|CallParentFunction OtherActor))

(event EventOnStateChanged
  (params (NewState :type EAIState%20Enum :default "Idle"))
  (|CallParentFunction NewState)
  (Rendering|Components|TextRender|SetText (Variables|/Game/UI/WBP_GuardState.WBP_GuardState_C|GetAlertedText (.AsWBP%20Guard%20State (Utilities|Casting|CastToWBP_GuardState (UserInterface|GetUserWidgetObject (Variables|Default|GetWidget))))) (Utilities|Select :Index NewState :Idle "" :Suspicious "?" :Alerted "!")))

(event EventTick
  (params (DeltaSeconds :type Float%20%28single-precision%29))
  (|CallParentFunction DeltaSeconds) ; This node is disabled and will not be called.\nDrag off pins to build functionality.
)

(fn ConstructionScript
  (|CallParentFunction))