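; BP_GameMOde is the game mode Blueprint that shows the end-of-mission screen.
; OnMissionCompleted creates a WBP_GameOver widget with the MissionSuccess result and adds it to the viewport.
; OverlapExtractionNoItem is an empty event.
; Disconnected nodes hold a timed missing-item message and a camera blend to BP_SpectatingViewpoint, neither of which runs.
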(event EventBeginPlay)

(event EventTick
  (params (DeltaSeconds :type Float%20%28single-precision%29)))

(event EventOnMissionCompleted
  (params (InstigatorPawn :type Pawn%20Object%20Reference) (bMissionSuccess :type Boolean))
  (Utilities|FlowControl|Sequence
    (:then_0
      (bind _returnvalue (UserInterface|CreateWidget "/Game/UI/WBP_GameOver.WBP_GameOver_C" 0 bMissionSuccess))
      (UserInterface|Viewport|AddtoViewport _returnvalue 0)
      (Widget|SetVisibility _returnvalue "Visible"))))

(event EventOverlapExtractionNoItem
  (params (InstigatorPawn :type Pawn%20Object%20Reference)))

(fn ConstructionScript)