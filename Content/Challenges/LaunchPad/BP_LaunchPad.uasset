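; BP_LaunchPad is a launch pad actor that flings characters and static mesh actors that overlap its box trigger.
; On overlap it spawns a gold ore aura particle effect at the pad.
; Static mesh actors get a forward and upward velocity-change impulse on their mesh component.
; Characters are launched along the pad's forward direction pitched up 45 degrees, overriding their current velocity.
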(event OnComponentBeginOverlap(Box)
  (params (OverlappedComponent :type Primitive%20Component%20Object%20Reference) (OtherActor :type Actor%20Object%20Reference) (OtherComp :type Primitive%20Component%20Object%20Reference) (OtherBodyIndex :type Integer) (bFromSweep :type Boolean) (SweepResult :type Hit%20Result%20Structure%20%28by%20ref%29))
  (bind _returnvalue (Transformation|GetActorForwardVector))
  (bind _returnvalue_2 (Transformation|GetActorRotation))
  (bind _returnvalue_3 (* _returnvalue 1.75e+03))
  (Effects|SpawnEmitteratLocation "/Game/Effects/P_gold_ore_aura.P_gold_ore_aura" (Transformation|GetActorLocation))
  (bind _asstatic_mesh_actor (Utilities|Casting|CastToStaticMeshActor OtherActor)
    (:then
      (Physics|AddImpulse (Variables|/Script/Engine.StaticMeshActor|GetStaticMeshComponent _asstatic_mesh_actor) (Math|Vector|MakeVector (.x _returnvalue_3) (.y _returnvalue_3) 1.5e+03) "None" true))
    (:CastFailed
      (bind _ascharacter (Utilities|Casting|CastToCharacter OtherActor))
      (Character|LaunchCharacter _ascharacter (* (Math|Rotator|GetRotationXVector (Math|Rotator|MakeRotator (.roll _returnvalue_2) (+ (.pitch _returnvalue_2) 45.0) (.yaw _returnvalue_2))) 1.5e+03) true true))))

(event EventBeginPlay)

(event Collision|EventActorBeginOverlap
  (params (OtherActor :type Actor%20Object%20Reference)))

(event EventTick
  (params (DeltaSeconds :type Float%20%28single-precision%29)))

(fn ConstructionScript)